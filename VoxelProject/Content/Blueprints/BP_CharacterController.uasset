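; Player character with Enhanced Input walk, look and jump, plus a debug hotbar for editing voxel terrain.
; Number keys set the hotbar index shown in WBP_DebugHotbar, and only the first slot has a mouse action.
; That slot line-traces from the camera to remove (left click) or add (right click) voxel spheres on a hit VoxelBase, with radius adjusted by mouse wheel.
; The 3 key is bound twice, setting two different indices.
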(event `Key|RightMouseButton`
  (params (Key :type "Key Structure"))
  ; mouse input right click
  (:`Pressed`
    (switch `int` (`self.hotbarCurrentIndex`)
      (:`0`
        (`self.voxel sphere` false)))))

(event `Key|LeftMouseButton`
  (params (Key :type "Key Structure"))
  ; mouse input left click
  (:`Pressed`
    (switch `int` (`self.hotbarCurrentIndex`)
      (:`0`
        (`self.voxel sphere` true)))))

(event `InputAxisKey|MouseWheelAxis`
  (params (AxisValue :type "Float (single-precision)"))
  (set `self.chunkSizeEffect` (+ (* AxisValue 10.0) (`self.chunkSizeEffect`))))

(event `Key|E`
  (params (Key :type "Key Structure"))
  (:`Pressed`
    (`KismetSystemLibrary.PrintString` (`KismetStringLibrary.Conv_DoubleToString` (`self.chunkSizeEffect`)))))

(event `Key|One`
  (params (Key :type "Key Structure"))
  ; set hotbar index
  (:`Pressed`
    (set `self.hotbarCurrentIndex` 0)
    (`/Game/Blueprints/WBP_DebugHotbar.SetActiveIndex` (`self.hotbar`) (stale `Key|Four` _output_get) :!label _label)))

(event `self.ReceiveBeginPlay`
  (bind _returnvalue (`|CreateWidget` "/Game/Blueprints/WBP_DebugHotbar.WBP_DebugHotbar_C"))
  (bind _output_get (set `self.hotbar` _returnvalue))
  (`UserWidget.AddToViewport` _output_get 0)
  ; Input Mapping Context
  (bind _asplayer_controller (cast `PlayerController` (`self.GetController`)))
  (`EnhancedInputSubsystemInterface.AddMappingContext` (pcsubsystem `EnhancedInputLocalPlayerSubsystem` _asplayer_controller) "/Game/Input/IMC_Character.IMC_Character" 0 (struct)))

(event `Key|Two`
  (params (Key :type "Key Structure"))
  ; set hotbar index
  (:`Pressed`
    (set `self.hotbarCurrentIndex` 1)
    (goto _label)))

(event `Key|Three`
  (params (Key :type "Key Structure"))
  ; set hotbar index
  (:`Pressed`
    (set `self.hotbarCurrentIndex` 2)
    (goto _label)))

(event `Key|Three`
  (params (Key :type "Key Structure"))
  ; set hotbar index
  (:`Pressed`
    (set `self.hotbarCurrentIndex` 3)
    (goto _label)))

(event `EnhancedInput|/Game/Input/IA_Look`
  (params (ActionValue :type "Vector2D Structure") (ElapsedSeconds :type "Float (double-precision)") (TriggeredSeconds :type "Float (double-precision)") (InputAction :type "InputAction Object Reference" :default "/Game/Input/IA_Look.IA_Look"))
  ; Camera Look
  (:`Triggered`
    (`self.AddControllerYawInput` ActionValue_X)
    (`self.AddControllerPitchInput` ActionValue_Y)))

(event `Key|Four`
  (params (Key :type "Key Structure"))
  ; set hotbar index
  (:`Pressed`
    (bind _output_get (set `self.hotbarCurrentIndex` 4))
    (goto _label)))

(event `EnhancedInput|/Game/Input/IA_Walk`
  (params (ActionValue :type "Vector2D Structure") (ElapsedSeconds :type "Float (double-precision)") (TriggeredSeconds :type "Float (double-precision)") (InputAction :type "InputAction Object Reference" :default "/Game/Input/IA_Walk.IA_Walk"))
  ; Player Movement
  (:`Triggered`
    (`self.AddMovementInput` (`self.GetActorRightVector`) ActionValue_X)
    (`self.AddMovementInput` (`self.GetActorForwardVector`) ActionValue_Y)))

(event `EnhancedInput|/Game/Input/IA_Jump`
  (params (ActionValue :type Boolean) (ElapsedSeconds :type "Float (double-precision)") (TriggeredSeconds :type "Float (double-precision)") (InputAction :type "InputAction Object Reference" :default "/Game/Input/IA_Jump.IA_Jump"))
  ; Player Jumping
  (:`Triggered`
    (`self.Jump`)))

(fn `UserConstructionScript`)

(fn `voxel sphere`
  (params (`left click` :type Boolean))
  (bind _returnvalue (`GameplayStatics.GetPlayerCameraManager` 0))
  (bind _chunksizeeffect (`self.chunkSizeEffect`))
  (bind _returnvalue_2 (`PlayerCameraManager.GetCameraLocation` _returnvalue))
  (bind _outhit (`KismetSystemLibrary.LineTraceSingle` _returnvalue_2 (+ _returnvalue_2 (* (`KismetMathLibrary.GetForwardVector` (`PlayerCameraManager.GetCameraRotation` _returnvalue)) (`self.rayMaxDis`))) "TraceTypeQuery1"))
  (bind (_bblockinghit _binitialoverlap _time _distance _location _impactpoint _normal _impactnormal _physmat _hitactor) (`GameplayStatics.BreakHitResult` _outhit))
  (bind _asvoxel_base (cast `VoxelBase` _hitactor)
    (:`then`
      (if `left click`
        (`Voxeleditinglibrary.RemoveVoxelsInSphere` _asvoxel_base _impactpoint _chunksizeeffect)
        (else
          (`Voxeleditinglibrary.AddVoxelsInSphere` _asvoxel_base _impactpoint _chunksizeeffect)))
      (`KismetSystemLibrary.PrintString` "hit the thing!"))
    (:`CastFailed`
      (`KismetSystemLibrary.PrintString` "didnt hit the thing"))))